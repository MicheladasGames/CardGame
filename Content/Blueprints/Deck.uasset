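; Deck actor for an Exploding Kittens-style card game, dealing cards to player 0's PuzzlePlayerCharacter.
; On BeginPlay it fills the deck from the CardTypes data table using four-player counts and random card images, then shuffles.
; The opening hand takes seven cards, sending Exploding and Defuse draws to the bottom of the deck, then adds an extra Defuse.
; Clicking the Cards component draws the top card for player 0.
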(event `self.ReceiveBeginPlay`
  ;[1 1 1] Build Deck for 4 players
  (bind _outrownames (`DataTableFunctionLibrary.GetDataTableRowNames` "/Game/CardTypes.CardTypes"))
  (for _array_element _outrownames
    (bind _returnvalue (`|GetDataTableRow` "/Game/CardTypes.CardTypes" _array_element)
      (:`then`
        (`self.addCardToDeck` _returnvalue))))
  (`KismetArrayLibrary.Array_Shuffle` (`self.deck`))
  (`self.ce_get_first_hand`))

(event `self.Cards.OnClicked`
  (params (TouchedComponent :type "PrimitiveComponent Object Reference") (ButtonPressed :type "Key Structure"))
  (bind _deck (`self.deck`))
  ;[1 1 1] Get First Card of Deck and give it to player 0
  (if (> (`KismetArrayLibrary.Array_Length` _deck) 0)
    (set `self._selectedCard` (`|GetArrayItem` _deck))
    (`KismetArrayLibrary.Array_Remove` (`self.deck`))
    (bind _aspuzzle_player_character (cast `/Game/PuzzleBP/Blueprints/PuzzlePlayerCharacter` (`GameplayStatics.GetPlayerCharacter` 0)))
    (`/Game/PuzzleBP/Blueprints/PuzzlePlayerCharacter.ce_add_card` _aspuzzle_player_character (`self._selectedCard`))))

(event `ce_get_first_hand`
  (bind __selectedcard_cardtype (break `/Game/CardStruct` (`self._selectedCard`)))
  (bind __initialhandofcard (`self._initialHandOfCard`))
  ;[1 1 1] Get First Card of Deck and give it to player 0
  (`KismetArrayLibrary.Array_Clear` __initialhandofcard)
  (while (< (`KismetArrayLibrary.Array_Length` __initialhandofcard) 7)
    (set `self._selectedCard` (`|GetArrayItem` (`self.deck`)))
    (`KismetArrayLibrary.Array_Remove` (`self.deck`))
    (switch `/Game/CardType` __selectedcard_cardtype
      (:`NewEnumerator0`
        ;;[1 1 1] First Hand Cannot include Defuse or Exploding
        (`KismetArrayLibrary.Array_Append` (`self.deck`) (`|MakeArray` (`self._selectedCard`)) :!label _label))
      (:`NewEnumerator1`
        (goto _label))
      (:`NewEnumerator2`
        (`KismetArrayLibrary.Array_Append` (`self._initialHandOfCard`) (`|MakeArray` (`self._selectedCard`)) :!label _label_2))
      (:`NewEnumerator3`
        (goto _label_2))
      (:`NewEnumerator4`
        (goto _label_2))
      (:`NewEnumerator5`
        (goto _label_2))
      (:`NewEnumerator6`
        (goto _label_2))
      (:`NewEnumerator7`
        (goto _label_2))
      (:`NewEnumerator8`
        (goto _label_2))
      (:`NewEnumerator9`
        (goto _label_2))
      (:`NewEnumerator10`
        (goto _label_2))
      (:`NewEnumerator11`
        (goto _label_2))
      (:`NewEnumerator12`
        (goto _label_2))))
  ;;[1 1 1] Give 7 Cards to Player 0 + 1 extra Defuse
  (`KismetArrayLibrary.Array_Append` (`self._initialHandOfCard`) (`|MakeArray` (make `/Game/CardStruct` "NewEnumerator1" "Extra Defuse" "{ Put your last drawn card back into the deck }")))
  (bind _aspuzzle_player_character (cast `/Game/PuzzleBP/Blueprints/PuzzlePlayerCharacter` (`GameplayStatics.GetPlayerCharacter` 0)))
  (`/Game/PuzzleBP/Blueprints/PuzzlePlayerCharacter.ce_initial_cards` _aspuzzle_player_character (`self._initialHandOfCard`)))

(fn `addCardToDeck`
  (params (card :type "/Game/CardTypeStruct Structure"))
  (bind _image (`self.getRandomImage` card_CardImage_15_33667DF43F44FD90769A448EC6A74D11))
  (for _ (range 1 (+ card_CardNumber4Players_19_8F3426AF7F4791C47CD1F1960927FFE9 1))
    (`KismetArrayLibrary.Array_Append` (`self.deck`) (`|MakeArray` (make `/Game/CardStruct` card_CardType_16_689194534B401D57E1C76089AEBFAD54 card_CardTitle_13_5FCB7ED1CF40D81A682A838926BA2C5B card_CardDescription_14_F7EEBD0C2B49D3B5EFDBF3B658F7231D _image)))))

(fn `getRandomImage`
  (params (images :type "Array of Texture2D Object Reference"))
  (returns (image :type "Texture2D Object Reference"))
  (return (`|GetArrayItem` images (`KismetMathLibrary.RandomIntegerInRange` 0 (- (`KismetArrayLibrary.Array_Length` images) 1)))))

(fn `UserConstructionScript`)